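; Multiplayer game state Blueprint, going by its name, that spawns or respawns a player's character.
; SpawnPlayer destroys the current pawn, then spawns one of two first-character variants according to the BP_PC_Multi controller's PlayerSelectedPC.
; RandomPlayerStart places it at one of the first two PlayerStarts found.
; Authority possesses the new pawn; both remote branches share one ClientPossess call that always receives the EM variant.
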(event EventBeginPlay)

(event EventTick
  (params (DeltaSeconds :type Float%20%28single-precision%29)))

(fn ConstructionScript)

(fn SpawnPlayer
  (params (Player%20Controller :type Player%20Controller%20Object%20Reference))
  (bind _returnvalue (Pawn|GetControlledPawn Player%20Controller))
  (Utilities|IsValid _returnvalue
    (:Is%20Valid
      (Actor|DestroyActor _returnvalue))
    (:Is%20Not%20Valid
      _))
  (bind _asbp_pc_multi (Utilities|Casting|CastToBP_PC_Multi Player%20Controller))
  (if (== (Variables|/Game/Multiplayer/Blueprints/BP_PC_Multi.BP_PC_Multi_C|GetPlayerSelectedPC _asbp_pc_multi) 0)
    (bind _returnvalue_2 (Game|SpawnActorfromClass "/Game/Multiplayer/Blueprints/BP_FirstChr2.BP_FirstChr2_C" (CallFunction|RandomPlayerStart) "AdjustIfPossibleButAlwaysSpawn" "MultiplyWithRoot" 0 0))
    (Variables|Default|SetPawnPosses _returnvalue_2)
    (Networking|SwitchHasAuthority
      (:Authority
        (Pawn|Possess Player%20Controller _returnvalue_2))
      (:Remote
        (Default|ClientPossess _asbp_pc_multi (stale _returnvalue_3) :!label _label)))
    (elif (== (Variables|/Game/Multiplayer/Blueprints/BP_PC_Multi.BP_PC_Multi_C|GetPlayerSelectedPC _asbp_pc_multi) 1)
      (bind _returnvalue_3 (Game|SpawnActorfromClass "/Game/Multiplayer/Blueprints/BP_FirstChr2_EM.BP_FirstChr2_EM_C" (CallFunction|RandomPlayerStart) "AdjustIfPossibleButAlwaysSpawn" "MultiplyWithRoot" 0 0))
      (Networking|SwitchHasAuthority
        (:Authority
          (Pawn|Possess Player%20Controller _returnvalue_3))
        (:Remote
          (goto _label))))))

(fn RandomPlayerStart
  (bind _outactors (Actor|GetAllActorsOfClass "/Script/Engine.PlayerStart"))
  (return (Transformation|GetActorTransform (Utilities|Array|Get(acopy) _outactors (Math|Random|RandomInteger 2)))))