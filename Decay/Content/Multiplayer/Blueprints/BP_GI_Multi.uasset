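; Multiplayer game instance Blueprint that hosts and joins online sessions for the first local player.
; CreateSession creates an eight-connection LAN session, prints the game mode name, then opens Lvl_FirstPerson as a listen server.
; JoinSession searches for up to five sessions and joins the first result without checking that the list has entries.
; Neither flow handles failure.
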(event Custom|Create%20Session
  (|Session (Game|GetPlayerController 0) 8 true true
    (:OnSuccess
      (Development|PrintString (Utilities|GetDisplayName (Game|GetGameMode)))
      (Game|OpenLevel(byObjectReference) "/Game/Multiplayer/Lvl_FirstPerson.Lvl_FirstPerson" true "?listen"))))

(event Custom|Join%20Session
  (bind _returnvalue (Game|GetPlayerController 0))
  (bind _results (|FindSessions _returnvalue 5 false false)
    (:OnSuccess
      (|JoinSession _returnvalue (Utilities|Array|Get(acopy) _results)))))