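; Multiplayer player state Blueprint whose only working logic looks up the team of a hit player.
; TeamChecker calls F_TeamChecker, which checks the Player tag, casts to BP_FirstChr2 and returns CurrentTeam from its BP_PC_Multi controller, printing debug strings on failed casts.
; Damage, death and health replication handlers are empty stubs, and a leftover cast chain in the event graph never runs.
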(event Custom|MC_AnyDamage)

(event Custom|MC_Death2)

(event Custom|TeamChecker
  (params (Hit%20Actor :type Actor%20Object%20Reference))
  (CallFunction|FTeamChecker Hit%20Actor))

(fn ConstructionScript)

(fn ROSAnyDamage
  (params (Damage1 :type Float%20%28double-precision%29) (Damage%20Type1 :type Damage%20Type%20Object%20Reference) (Instigated%20By1 :type Controller%20Object%20Reference) (Damage%20Causer1 :type Actor%20Object%20Reference)))

(fn OnRepCharacterHealth)

(fn FTeamChecker
  (params (Hit%20Actor :type Actor%20Object%20Reference))
  (if (Actor|ActorHasTag Hit%20Actor "Player")
    (bind _asbp_first_chr_2 (Utilities|Casting|CastToBP_FirstChr2 Hit%20Actor)
      (:then
        (bind _asbp_pc_multi (Utilities|Casting|CastToBP_PC_Multi (Pawn|GetController _asbp_first_chr_2))
          (:then
            (return (Variables|/Game/Multiplayer/Blueprints/BP_PC_Multi.BP_PC_Multi_C|GetCurrentTeam _asbp_pc_multi)))
          (:CastFailed
            (Development|PrintString "Hello4"))))
      (:CastFailed
        (Development|PrintString "Hello3")))))