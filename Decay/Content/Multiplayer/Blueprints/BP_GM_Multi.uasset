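; Multiplayer game mode that assigns players to one of two teams and spawns their selected character.
; On PostLogin, it adds the player to the smaller team (Team 2 on a tie) and reports it through BP_PC_Multi.
; SpawnPlayer destroys any current pawn, then possesses a character chosen by PlayerSelectedPC, placed at one of the first two PlayerStarts at random.
; CharacterSelectBranches always spawns BP_FirstChr2 for NewPlayer, ignoring its PlayerController input.
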(event EventPostLogin
  (params (NewPlayer :type Player%20Controller%20Object%20Reference))
  (bind _output_get (Variables|Default|SetNew%20Player NewPlayer))
  ;[0.15 0.15 0.15 0.5 30] This code assigns the player a team upon logging in. If there are more people on Team 1, it will place the connecter on Team 2 and vice versa.
  (if (>= (Utilities|Array|Length (Variables|Default|GetTeam1Players)) (Utilities|Array|Length (Variables|Default|GetTeam2Players)))
    (Utilities|Array|Add (Variables|Default|GetTeam2Players) _output_get)
    (bind _output_get_2 (Variables|Default|SetTeam 2))
    (bind _asbp_pc_multi (Utilities|Casting|CastToBP_PC_Multi _output_get))
    (Utilities|IsValid _asbp_pc_multi
      (:Is%20Valid
        (Default|TeamStatus _asbp_pc_multi _output_get_2)))
    (else
      (Utilities|Array|Add (Variables|Default|GetTeam1Players) _output_get)
      (bind _output_get_3 (Variables|Default|SetTeam 1))
      (bind _asbp_pc_multi_2 (Utilities|Casting|CastToBP_PC_Multi _output_get))
      (Utilities|IsValid _asbp_pc_multi_2
        (:Is%20Valid
          (Default|TeamStatus _asbp_pc_multi_2 _output_get_3))))))

(fn ConstructionScript)

(fn RandomPlayerStart
  (bind _outactors (Actor|GetAllActorsOfClass "/Script/Engine.PlayerStart"))
  (return (Transformation|GetActorTransform (Utilities|Array|Get(acopy) _outactors (Math|Random|RandomInteger 2)))))

(fn SpawnPlayer
  (params (Player%20Controller :type Player%20Controller%20Object%20Reference))
  (bind _returnvalue (Pawn|GetControlledPawn Player%20Controller))
  ;[0.15 0.15 0.15 0.5] This code checks if the player has a pawn, if it does, it destroys the pawn and executes the rest of the code. Otherwise, it simply creates a pawn for the player and has them possess it.
  (Utilities|IsValid _returnvalue
    (:Is%20Valid
      (Actor|DestroyActor _returnvalue))
    (:Is%20Not%20Valid
      _))
  (bind _asbp_pc_multi (Utilities|Casting|CastToBP_PC_Multi Player%20Controller))
  (if (== (Variables|/Game/Multiplayer/Blueprints/BP_PC_Multi.BP_PC_Multi_C|GetPlayerSelectedPC _asbp_pc_multi) 0)
    (bind _returnvalue_2 (Game|SpawnActorfromClass "/Game/Multiplayer/Blueprints/BP_FirstChr2.BP_FirstChr2_C" (CallFunction|RandomPlayerStart) "AdjustIfPossibleButAlwaysSpawn" "MultiplyWithRoot" 0 0))
    (Pawn|Possess Player%20Controller _returnvalue_2)
    (elif (== (Variables|/Game/Multiplayer/Blueprints/BP_PC_Multi.BP_PC_Multi_C|GetPlayerSelectedPC _asbp_pc_multi) 1)
      (bind _returnvalue_3 (Game|SpawnActorfromClass "/Game/Multiplayer/Blueprints/BP_FirstChr2_EM.BP_FirstChr2_EM_C" (CallFunction|RandomPlayerStart) "AdjustIfPossibleButAlwaysSpawn" "MultiplyWithRoot" 0 0))
      (Pawn|Possess Player%20Controller _returnvalue_3))))

(fn CharacterSelectBranches
  (params (Player%20Controller :type Player%20Controller%20Object%20Reference))
  (bind _returnvalue (Game|SpawnActorfromClass "/Game/Multiplayer/Blueprints/BP_FirstChr2.BP_FirstChr2_C" (CallFunction|RandomPlayerStart) "AdjustIfPossibleButAlwaysSpawn" "MultiplyWithRoot" 0 0))
  (Pawn|Possess (Variables|Default|GetNew%20Player) _returnvalue))